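; HUD for the hex map that sets up the selection and builder actors, the main widget layout, and a starter town hall with two houses.
; HighlightHex and ClearHighlightedHexes recycle a pre-spawned pool of hex decals, growing it when empty.
; Keys trigger GameInstance turn calls or highlight construct locations of the structure under the mouse, green or red if blocked.
; Tick draws debug arrows linking root structures to their BroadcastTo structures.
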(event EventBeginPlay
  (bind _returnvalue (Game|GetPlayerController 0))
  (bind _returnvalue_2 (Math|Transform|MakeTransform "0, 0, 0"))
  (Utilities|FlowControl|Sequence
    (:then_0
      (bind _asgi_potl (Utilities|Casting|CastToGI_POTL (Game|GetGameInstance)))
      (Variables|Default|SetGameInstance _asgi_potl))
    (:then_4
      ;[1 1 1] Decals
      (Utilities|FlowControl|Sequence
        (:then_0
          (for _index (range 0 199)
            (bind _returnvalue_3 (Game|SpawnActorfromClass "/Game/Blueprint/Actor/BP_HexDecal.BP_HexDecal_C" (Math|Transform|MakeTransform "0.000000, 0, 0" "-90.000000,0.000000, 0" "500.000000,142.000000,124.000000") "AlwaysSpawn" 0 0))
            (Rendering|SetActorHiddenInGame _returnvalue_3 true)
            (Utilities|Array|Add (Variables|Decals|GetFreeHighlightDecals) _returnvalue_3)))
        (:then_1
          ;[1 1 1] Spawn the Selection Hex actor
          (bind _returnvalue_4 (Game|SpawnActorfromClass "/Game/Blueprint/Actor/BP_Hex.BP_Hex_C" _returnvalue_2 "AdjustIfPossibleButDontSpawnIfColliding" 0 0))
          (Variables|Default|SetHex _returnvalue_4)
          (Game|SpawnActorfromClass "/Game/Blueprint/Actor/Util/BP_BuilderStructure.BP_BuilderStructure_C" _returnvalue_2 "AdjustIfPossibleButDontSpawnIfColliding" 0 0))))
    (:then_5
      ;[1 1 1] Widgets
      (Utilities|FlowControl|Sequence
        (:then_0
          (bind _returnvalue_5 (UserInterface|CreateWidget "/Game/Blueprint/HUD/Layout/Widget_MainLayout.Widget_MainLayout_C" _returnvalue))
          (Utilities|FlowControl|Sequence
            (:then_0
              (bind _returnvalue_6 (UserInterface|CreateWidget "/Game/Blueprint/HUD/Widgets/Widget_Builder.Widget_Builder_C" _returnvalue))
              (Widget|Panel|AddChild (Variables|/Game/Blueprint/HUD/Layout/Widget_MainLayout.Widget_MainLayout_C|GetNamedSlot_100 _returnvalue_5) _returnvalue_6))
            (:then_1
              (bind _returnvalue_7 (UserInterface|CreateWidget "/Game/Blueprint/HUD/Widgets/Widget_SelectedHex.Widget_SelectedHex_C" _returnvalue))
              (Widget|Panel|AddChild (Variables|/Game/Blueprint/HUD/Layout/Widget_MainLayout.Widget_MainLayout_C|GetNamedSlot_76 _returnvalue_5) _returnvalue_7))
            (:then_2
              (bind _returnvalue_8 (UserInterface|CreateWidget "/Game/Blueprint/HUD/Widgets/Widget_StructureEditor.Widget_StructureEditor_C" _returnvalue))
              (Widget|Panel|AddChild (Variables|/Game/Blueprint/HUD/Layout/Widget_MainLayout.Widget_MainLayout_C|GetNamedSlot_316 _returnvalue_5) _returnvalue_8))
            (:then_3
              (UserInterface|Viewport|AddtoViewport _returnvalue_5 0))))))
    (:then_6
      (Utilities|FlowControl|Sequence
        (:then_0
          (Utilities|FlowControl|Delay 0.0)
          (bind _returnvalue_9 (Default|PlantStructure (Variables|Default|GetGameInstance) "0,-17.000000,17.000000" "TownHall" "None" 0 false))
          (Default|PlantStructure (Variables|Default|GetGameInstance) "1.000000,-20.000000,19.000000" "House" "None" _returnvalue_9 false)
          (Default|PlantStructure (Variables|Default|GetGameInstance) "-5.000000,-15.000000,20.000000" "House" "None" _returnvalue_9 false))
        (:then_1
          (Input|EnableInput (Game|GetPlayerController 0)))))))

(event Collision|EventActorBeginOverlap
  (params (OtherActor :type Actor%20Object%20Reference)))

(event EventTick
  (params (DeltaSeconds :type Float%20%28single-precision%29))
  (Utilities|FlowControl|Sequence
    (:then_0
      (for _array_element (Variables|/Script/POTL.POTLGameInstance|GetRootStructures (Variables|Default|GetGameInstance))
        (for _array_element_2 (Variables|/Script/POTL.POTLStructure|GetBroadcastTo _array_element)
          (Rendering|Debug|DrawDebugArrow (+ (Transformation|GetActorLocation _array_element_2) "0, 0,250.000000") (+ (Transformation|GetActorLocation _array_element) "0, 0,250.000000") 2e+02 "(R=0.000000,G=0.472928,B=1.000000,A=1.000000)" 0.0))))))

(event Input|KeyboardEvents|T
  (params (Key :type Key%20Structure :default "AnyKey"))
  ;[1 1 1] Toogle debug
  (:Pressed
    (Variables|Default|SetToogleDebug (not (Variables|Default|GetToogleDebug)))
    (CallFunction|ClearHighlightedHexes (Variables|Default|GetAttachSpotsHighlights))
    (bind (_found _hex) (Default|MousePostoHex (Variables|Default|GetGameInstance)))
    (if _found
      (Development|PrintString (Utilities|GetDisplayName (.AttachedBuilding (Utilities|Struct|BreakST_Hex _hex))) true true "(R=0.000000,G=0.660000,B=1.000000,A=1.000000)" 15.0)
      (bind _returnvalue (Class|POTLGameInstance|GetConstructLocations (Variables|Default|GetGameInstance) (.AttachedBuilding (Utilities|Struct|BreakST_Hex _hex)) true))
      (for _array_element _returnvalue
        (CallFunction|HighlightHex _array_element (Variables|Default|GetAttachSpotsHighlights) (Utilities|Select :Index (Math|Conversions|ToInteger(Boolean) (.Blocked (Utilities|Struct|BreakST_ConstructLocation (.ConstructInfo (Utilities|Struct|BreakST_Hex _array_element))))) :Option%200 "Green" :Option%201 "Red"))))))

(event Input|KeyboardEvents|N
  (params (Key :type Key%20Structure :default "AnyKey"))
  (:Released
    (Class|POTLGameInstance|SwitchTurn (Variables|Default|GetGameInstance))))

(event Input|KeyboardEvents|Y
  (params (Key :type Key%20Structure :default "AnyKey"))
  (:Released
    (Class|POTLGameInstance|NewTurn (Variables|Default|GetGameInstance) 0.0)))

(event Input|MouseEvents|LeftMouseButton
  (params (Key :type Key%20Structure :default "AnyKey")))

(fn ConstructionScript)

(fn HighlightHex
  (params (Hex :type ST%20Hex%20Structure) (HighlightList :type Array%20of%20BP%20Hex%20Decal%20Object%20References) (Type :type Name))
  (bind _freehighlightdecals (Variables|Decals|GetFreeHighlightDecals))
  (bind _item (Utilities|Array|Get(acopy) _freehighlightdecals))
  (if (== (Utilities|Array|Length _freehighlightdecals) 0)
    (for _index (range 0 249)
      (bind _returnvalue (Game|SpawnActorfromClass "/Game/Blueprint/Actor/BP_HexDecal.BP_HexDecal_C" (Math|Transform|MakeTransform "0.000000, 0, 0" "-90.000000,0.000000, 0" "500.000000,142.000000,124.000000") "AlwaysSpawn" (Game|GetPlayerController 0) 0))
      (Rendering|SetActorHiddenInGame _returnvalue true)
      (Utilities|Array|Add (Variables|Decals|GetFreeHighlightDecals) _returnvalue)))
  (Transformation|SetActorLocation _item (.Location (Utilities|Struct|BreakST_Hex Hex)) false false)
  (Rendering|SetActorHiddenInGame _item false)
  (Utilities|Array|Add HighlightList _item)
  (Default|ChangeType _item Type)
  (Utilities|Array|RemoveIndex _freehighlightdecals))

(fn ClearHighlightedHexes
  (params (LightlightList :type Array%20of%20BP%20Hex%20Decal%20Object%20References))
  (for _array_element LightlightList
    (Transformation|SetActorLocation _array_element "0, 0, 0" false false)
    (Rendering|SetActorHiddenInGame _array_element true)
    (Utilities|Array|Add (Variables|Decals|GetFreeHighlightDecals) _array_element))
  (Utilities|Array|Clear LightlightList))

(fn DrawDebug2
  (for _array_element (Variables|/Script/POTL.POTLGameInstance|GetHexes (Variables|Default|GetGameInstance))
    (Utilities|FlowControl|Sequence
      (:then_1
        (for _array_element_2 (Utilities|Array|MakeArray (.Point0 (Utilities|Struct|BreakST_Hex _array_element)) (.Point1 (Utilities|Struct|BreakST_Hex _array_element)) (.Point2 (Utilities|Struct|BreakST_Hex _array_element)) (.Point3 (Utilities|Struct|BreakST_Hex _array_element)) (.Point4 (Utilities|Struct|BreakST_Hex _array_element)) (.Point5 (Utilities|Struct|BreakST_Hex _array_element)))
          (Rendering|Debug|DrawDebugLine (.Location (Utilities|Struct|BreakST_Point _array_element_2)) (+ (.Location (Utilities|Struct|BreakST_Point _array_element_2)) "0, 0,50.000000") "(R=0.000000,G=0.127595,B=1.000000,A=1.000000)" 15.0 1e+01))))))