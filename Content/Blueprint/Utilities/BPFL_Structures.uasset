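; Blueprint function library of struct helpers for building, hex and state-object data.
; GetStateObjectById linearly searches a list for a matching Id and returns that entry's State, with the Index output fixed at 0.
; MakeBuildingStruct and MakeHexStruct rebuild STBuilding and STHex values by copying the fields of a passed-in building or hex, including attachments and hex coordinates.
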(fn GetStateObjectbyId
  (params (List :type Array%20of%20ST%20State%20Object%20Structures) (Id :type Name :default "None"))
  (bind _array_element (Utilities|Array|ForEachLoopwithBreak List)
    (:LoopBody
      (if (Utilities|Name|Equal(Name) (.Id (Utilities|Struct|BreakST_StateObject _array_element)) Id)
        (return (.State (Utilities|Struct|BreakST_StateObject _array_element)) 0)))))

(fn MakeBuildingStruct
  (params (OldBuilding :type ST%20Building%20Structure))
  (bind (_id _title _burnable _actorclass _attachto) (Utilities|Struct|BreakST_Building OldBuilding))
  (return (Utilities|Struct|MakeST_Building _id _title _burnable _actorclass _attachto)))

(fn MakeHexStruct
  (params (Old%20Hex :type ST%20Hex%20Structure))
  (bind (_location _rotation _point0 _point1 _point2 _point3 _point4 _point5 _remove _attachedbuilding _attachedactor _attachedmesh _hexcubecoords _hexoffsetcoords) (Utilities|Struct|BreakST_Hex Old%20Hex))
  (return (Utilities|Struct|MakeST_Hex _location _rotation _point0 _point1 _point2 _point3 _point4 _point5 _remove _attachedbuilding _attachedactor _attachedmesh _hexcubecoords _hexoffsetcoords)))