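; BPFL_Hex is a Blueprint function library of small general-purpose utility functions.
; ExistsInLevel treats an actor as present when its display name is non-empty, rather than using a validity check.
; PrintIntArray joins integers into a comma-separated string and prints it in a given color for debugging.
; GetPoint performs a bounds-checked lookup in a points array, returning the point with a found flag.
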(fn ExistsinLevel
  (params (Actor :type Actor%20Object%20Reference))
  (return (> (Utilities|String|Len (Utilities|GetDisplayName Actor)) 0)))

(fn PrintIntArray
  (params (NewParam :type Array%20of%20Integers) (Color :type Linear%20Color%20Structure))
  (for _array_element NewParam
    (LocalVariables|SetValue (Utilities|String|BuildString(Integer) (LocalVariables|GetValue) "" _array_element ", ")))
  (Development|PrintString 0 (LocalVariables|GetValue) true true Color))

(fn GetPoint
  (params (Points :type Array%20of%20ST%20Point%20Structures) (Index :type Integer :default 0))
  (bind _returnvalue (Utilities|Array|Length Points))
  (bind _returnvalue_2 (>= Index 0))
  (bind _returnvalue_3 (< Index _returnvalue))
  (bind _returnvalue_4 (and _returnvalue_3 _returnvalue_2))
  (if _returnvalue_4
    (return (Utilities|Array|Get(acopy) Points Index) _returnvalue_4)))