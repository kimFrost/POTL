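; BP_Building is a building actor that forms trees through an Attachments array, with debug drawing for living slots, build range and links.
; On TurnSwitched, a root building calls UpdateTree, which only recurses through attachments.
; Tick draws the TreeId above the actor.
; BeginPlay is empty: turn binding, Initialize's attachment search and the looping DrawDebugs timer are disconnected, and several functions are stubs.
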(event Custom|TurnSwitched
  (params (TurnsProgressed :type Integer))
  (if (Variables|Default|GetIsRoot)
    (Development|PrintString "BP_Building: TurnSwitched")
    (CallFunction|UpdateTree)))

(event Custom|CustomEvent_0
  (CallFunction|DrawDebugs 1.0))

(event EventBeginPlay)

(event Collision|EventActorBeginOverlap
  (params (OtherActor :type Actor%20Object%20Reference)))

(event EventTick
  (params (DeltaSeconds :type Float%20%28single-precision%29))
  (Rendering|Debug|DrawDebugString (+ (Transformation|GetActorLocation) "0, 0,300.000000") (Utilities|String|ToString(Name) (Variables|Default|GetTreeId)) 0 "(R=0.977886,G=0.000000,B=1.000000,A=1.000000)"))

(fn ConstructionScript)

(fn Initialize
  (if (not (> (Variables|Default|GetExtendBuildRange) 0))
    ;[1 1 1] Attach Self to "nearest"  building with extend range
    (bind _outactors (Actor|GetAllActorsOfClass "BP_Building_C"))
    (bind _array_element (Utilities|Array|ForEachLoopwithBreak _outactors :!label _label)
      (:LoopBody
        (if (> (Variables|BP_Building_C|GetExtendBuildRange _array_element) 0)
          (CallFunction|AttachBuilding self)
          (Development|PrintString (Utilities|GetDisplayName _array_element) true true "(R=0.691066,G=0.000000,B=1.000000,A=1.000000)")
          (goto _label Break))))))

(fn DrawDebugs
  (params (Time :type Float%20%28single-precision%29 :default 0.0))
  (bind _returnvalue (Math|Float|MakeLiteralFloat 1.0))
  (bind _self self)
  (bind _returnvalue_2 (Transformation|GetActorLocation _self))
  (Utilities|FlowControl|Sequence
    (:then_0
      (for _array_element (Variables|Default|GetDebugMeshes)
        (Components|DestroyComponent _array_element)))
    (:then_1
      (for (_array_element_2 _array_index) (Variables|Default|GetLivingSlots)
        (bind _returnvalue_3 (AddComponent|AddStaticMeshComponent false (Math|Transform|MakeTransform (Math|Vector|MakeVector 0.0 0.0 (* _array_index 25.0)))))
        (Components|StaticMesh|SetStaticMesh _returnvalue_3 "/Game/Meshes/DebugMesh.DebugMesh")
        (bind _returnvalue_4 (Rendering|Material|CreateDynamicMaterialInstance "/Game/Materials/M_Debug_Inst.M_Debug_Inst" :!class /Script/Engine.KismetMaterialLibrary))
        (Rendering|Material|SetVectorParameterValue _returnvalue_4 "Color" (Math|Color|SelectColor "(R=0.610346,G=1.000000,B=0.000000,A=1.000000)" "(R=1.000000,G=0.000000,B=0.687128,A=1.000000)" (Utilities|Name|Equal(Name) (.Id (Utilities|Struct|BreakST_Person (Utilities|Struct|BreakST_LivingSlot _array_element_2))) "None")) :!class /Script/Engine.MaterialInstanceDynamic)
        (Rendering|Material|SetMaterial _returnvalue_3 0 _returnvalue_4)
        (Utilities|Array|Add (Variables|Default|GetDebugMeshes) _returnvalue_3)))
    (:then_2
      (Class|KismetSystemLibrary|DrawDebugCylinder (+ _returnvalue_2 "0, 0,-500.000000") (+ _returnvalue_2 "0.000000,0.000000,500.000000") (+ (* (Variables|Default|GetExtendBuildRange) 255.0) 127.5) 12 "(R=0.208649,G=1.000000,B=0.019694,A=1.000000)" _returnvalue))
    (:then_3
      (for _array_element_3 (Variables|Default|GetAttachments)
        (Rendering|Debug|DrawDebugLine (Transformation|GetActorLocation self) (Transformation|GetActorLocation _array_element_3) "(R=0.360000,G=0.764947,B=1.000000,A=1.000000)" _returnvalue 5.0)))))

(fn UpdateTree
  ;[1 1 1] Resolve Attached buildings
  (for _array_element (Variables|Default|GetAttachments)
    ;[1 1 1] Resolve Attached Building Childs
    (CallFunction|UpdateTree _array_element)))

(fn ResetResources)

(fn AttachBuilding
  (params (Building :type BP%20Building%20Object%20Reference))
  (Utilities|Array|Add (Variables|Default|GetAttachments) Building))

(fn ToggleAttachSpots)