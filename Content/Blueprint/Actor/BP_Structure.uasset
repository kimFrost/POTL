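; Turn-based structure actor that forms a node in a resource tree linked through EmitTo and BroadcastTo.
; On game-instance turn events, only the root acts: it resolves the tree on a turn switch, and on a new turn allocates resources and respawns BP_ResourceFlow actors from its BroadcastTo structures.
; Tick optimizes allocations inside DrawDebugs, then draws free-resource bars, an EmitTo arrow and an in-range sphere.
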(event Custom|_OnNewTurn
  (params (Turn :type Float%20%28single-precision%29))
  (if (Variables|Default|GetIsRoot)
    (Class|POTLStructure|MakeTreeAllocations)
    (Class|POTLStructure|GetAllocationsasList)
    (bind _outactors (Actor|GetAllActorsOfClass "/Game/Blueprint/Actor/BP_ResourceFlow.BP_ResourceFlow_C"))
    (for _array_element _outactors
      (Actor|DestroyActor _array_element))
    (for _array_element_2 (Variables|Default|GetBroadcastTo)
      (bind _returnvalue (Class|POTLStructure|GetStructureResourceFlow _array_element_2))
      (Development|PrintString (Utilities|String|ToString(Integer) (Utilities|Array|Length _returnvalue)))
      (if (> (Utilities|Array|Length _returnvalue) 0)
        (Game|SpawnActorfromClass "/Game/Blueprint/Actor/BP_ResourceFlow.BP_ResourceFlow_C" (Math|Transform|MakeTransform (Transformation|GetActorLocation _array_element_2)) "Undefined" 0 "0.000000,0.000000,0.000000" (- (Transformation|GetActorLocation self) (Transformation|GetActorLocation _array_element_2)) -1 "Not Set" -1 _returnvalue)
        (Development|PrintString "Hello")))))

(event Custom|_OnTurnSwitched
  (params (Turn :type Float%20%28single-precision%29))
  (if (Variables|Default|GetIsRoot)
    (Class|POTLStructure|ResolveTree)))

(event EventUpdateConstrunction
  (|CallParentFunction))

(event EventBeginPlay
  (bind _asgi_potl (Utilities|Casting|CastToGI_POTL (Game|GetGameInstance)))
  (EventDispatchers|BindEventtoOnTurnSwitched _asgi_potl (delegate Custom|_OnTurnSwitched))
  (EventDispatchers|BindEventtoOnNewTurn _asgi_potl (delegate Custom|_OnNewTurn)))

(event Collision|EventActorBeginOverlap
  (params (OtherActor :type Actor%20Object%20Reference)))

(event EventTick
  (params (DeltaSeconds :type Float%20%28single-precision%29))
  (CallFunction|DrawDebugs 0.0))

(fn ConstructionScript)

(fn DrawDebugs
  (params (Time :type Float%20%28single-precision%29 :default 0.0))
  (bind _returnvalue (Math|Vector|MakeVector 0.0 0.0 2.5e+02))
  (bind _returnvalue_2 (Transformation|GetActorLocation))
  (bind _returnvalue_3 (+ _returnvalue_2 "0, 0,250.000000"))
  (Utilities|FlowControl|Sequence
    (:then_0
      ;[1 1 1] Resources - Free
      (Class|POTLStructure|OptimizeAllocatedResources))
    (:then_1
      (bind _returnvalue_4 (Class|POTLStructure|GetResourcesasList "Free"))
      (for (_array_element _array_index) _returnvalue_4
        (switch string (.Id (Utilities|Struct|BreakST_Resource _array_element))
          (:Wood
            (LocalVariables|Set%25_DrawDebugs_Color "(R=0.600000,G=0.278520,B=0.023094,A=1.000000)"))
          (:Stone
            (LocalVariables|Set%25_DrawDebugs_Color "(R=0.405000,G=0.376592,B=0.335321,A=1.000000)"))
          (:Plank
            (LocalVariables|Set%25_DrawDebugs_Color "(R=0.890000,G=0.000000,B=0.164208,A=1.000000)"))
          (:Wheat
            (LocalVariables|Set%25_DrawDebugs_Color "(R=0.980000,G=0.898639,B=0.225400,A=1.000000)"))
          (:Flour
            (LocalVariables|Set%25_DrawDebugs_Color "(R=0.935000,G=0.893907,B=0.832150,A=1.000000)"))
          (:Bread
            (LocalVariables|Set%25_DrawDebugs_Color "(R=0.870000,G=0.606517,B=0.363827,A=1.000000)")))
        (Class|KismetSystemLibrary|DrawDebugCylinder (+ _returnvalue_3 (Math|Vector|MakeVector (- (* _array_index 25.0) 1e+02) 0.0 0.0)) (+ _returnvalue_3 (Math|Vector|MakeVector (- (* _array_index 25.0) 1e+02) 0.0 (* (.Quantity (Utilities|Struct|BreakST_Resource _array_element)) 1e+01))) 1e+01 12 (LocalVariables|Get%25_DrawDebugs_Color) 0.0)
        (Rendering|Debug|DrawDebugString (+ _returnvalue_3 (Math|Vector|MakeVector (- (* _array_index 25.0) 1e+02) 0.0 (* (.Quantity (Utilities|Struct|BreakST_Resource _array_element)) 1e+01))) (Utilities|String|ToString(Integer) (.Quantity (Utilities|Struct|BreakST_Resource _array_element))) 0 "(R=1.000000,G=1.000000,B=1.000000,A=1.000000)")))
    (:then_2
      ;[1 1 1] Resources - Allocated - Text
      (for (_array_element_2 _array_index_2) 0
        _))
    (:then_3
      ;[1 1 1] EmitTo
      (bind _asbp_structure (Utilities|Casting|CastToBP_Structure (Variables|Default|GetEmitTo)))
      (Rendering|Debug|DrawDebugArrow (+ (Transformation|GetActorLocation) _returnvalue) (+ (Transformation|GetActorLocation _asbp_structure) _returnvalue) 5e+01 "(R=0.102843,G=0.000000,B=1.000000,A=1.000000)" 0.0))
    (:then_4
      (Rendering|Debug|DrawDebugSphere (+ (Math|Vector|MakeVector 0.0 0.0 2.5e+02) (Transformation|GetActorLocation)) 5e+01 12 (Math|Color|SelectColor "(R=0.000000,G=1.000000,B=0.047340,A=1.000000)" "(R=1.000000,G=0.077957,B=0.000000,A=1.000000)" (Variables|Default|GetInRangeOfEmitTo)) 0.0))))

(fn WriteData)

(fn ReadData
  (bind _returnvalue (Utilities|GetDataTableRow "/Game/Resources/Structures.Structures" (Variables|Default|GetStrutureRowName_Deprecated))))