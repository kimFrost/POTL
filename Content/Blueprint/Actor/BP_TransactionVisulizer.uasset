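; Actor that visualizes a transaction as a spline mesh stretched from its seller to its buyer.
; On BeginPlay it teleports to the Seller's location and sets the spline mesh end position to the offset toward the Buyer.
; It destroys itself if the Transaction is invalid and does not update the endpoints afterward.
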(event EventBeginPlay
  (bind _transaction (Variables|Default|GetTransaction))
  (bind _transaction_2 (Variables|Default|GetTransaction))
  (bind _seller (Variables|/Script/POTL.Transaction|GetSeller _transaction))
  (bind _buyer (Variables|/Script/POTL.Transaction|GetBuyer _transaction_2))
  (bind _returnvalue (Transformation|GetActorLocation _seller))
  (Utilities|IsValid _transaction
    (:Is%20Valid
      (Utilities|IsValid _seller
        (:Is%20Valid
          (Transformation|SetActorLocation _returnvalue false true)
          (Utilities|IsValid _buyer
            (:Is%20Valid
              (SplineMesh|SetEndPosition (Variables|Default|GetSplineMesh) (- (Transformation|GetActorLocation _buyer) _returnvalue) true))))))
    (:Is%20Not%20Valid
      (Actor|DestroyActor))))

(event Collision|EventActorBeginOverlap
  (params (OtherActor :type Actor%20Object%20Reference)))

(event EventTick
  (params (DeltaSeconds :type Float%20%28single-precision%29)))

(fn ConstructionScript)