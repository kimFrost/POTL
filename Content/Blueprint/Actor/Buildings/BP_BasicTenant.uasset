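; BP_BasicTenant is a tenant building actor that displays its residents' resource levels in the world.
; Each tick it writes the Food and Wealth values from its Residents data to two text render components.
; Disconnected debug prints for game mode time and Labor progress remain in the graph but never run.
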(event EventBeginPlay
  (|CallParentFunction))

(event Collision|EventActorBeginOverlap
  (params (OtherActor :type Actor%20Object%20Reference)))

(event EventTick
  (params (DeltaSeconds :type Float%20%28single-precision%29))
  (bind _residents (Variables|Default|GetResidents))
  (Rendering|Components|TextRender|SetText (Variables|Default|GetTextRender) (Utilities|Text|ToText(Float) (Variables|/Script/POTL.ResidentsComponent|GetFood _residents) "HalfToEven"))
  (Rendering|Components|TextRender|SetText (Variables|Default|GetTextRender1) (Utilities|Text|ToText(Float) (Variables|/Script/POTL.ResidentsComponent|GetWealth _residents) "HalfToEven")))

(fn ConstructionScript
  (|CallParentFunction))