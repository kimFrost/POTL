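; BP_Windmill is a building actor that continuously spins one of its meshes, StaticMesh1.
; Each Tick combines the mesh's relative rotation with a roll increment scaled by delta time, giving a constant, frame-rate-independent spin at a hardcoded speed.
; BeginPlay and the construction script only call their parent versions.
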(event EventBeginPlay
  (|CallParentFunction))

(event Collision|EventActorBeginOverlap
  (params (OtherActor :type Actor%20Object%20Reference)))

(event EventTick
  (params (DeltaSeconds :type Float%20%28single-precision%29))
  (bind _staticmesh1 (Variables|Default|GetStaticMesh1))
  (|CallParentFunction DeltaSeconds)
  (Transformation|SetRelativeRotation _staticmesh1 (Math|Rotator|CombineRotators (Variables|/Script/Engine.SceneComponent|GetRelativeRotation _staticmesh1) (Math|Rotator|MakeRotator (* DeltaSeconds 3e+01) 0.0 0.0)) false false))

(fn ConstructionScript
  (|CallParentFunction))