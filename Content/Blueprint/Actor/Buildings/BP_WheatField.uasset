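; Wheat field building actor that builds a patch of wheat and a spline-driven fence in its construction script.
; CreateWheat scatters an instanced static mesh over a fixed square grid centered on the actor, with random yaw and scale, independent of the fence shape.
; The fence spline is handed to a BP_Prop-SplineMesh child actor to generate meshes.
; The local CreateFence is not called, and AlignPointsToGrid is an empty stub.
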(fn ConstructionScript
  (|CallParentFunction)
  (CallFunction|AlignPointstoGrid)
  (CallFunction|CreateWheat)
  (bind _asbp_prop__spline_mesh (Utilities|Casting|CastToBP_Prop-SplineMesh (Variables|/Script/Engine.ChildActorComponent|GetChildActor (Variables|Default|GetFenceMeshes))))
  (Variables|/Game/Blueprint/Actor/Props/BP_Prop-SplineMesh.BP_Prop-SplineMesh_C|SetSpline _asbp_prop__spline_mesh (Variables|Default|GetFenceSpline))
  (Default|CreateSplineMeshes _asbp_prop__spline_mesh))

(fn CreateFence
  (bind _fencespline (Variables|Default|GetFenceSpline))
  (bind _returnvalue (Spline|GetNumberOfSplinePoints _fencespline))
  (if (Class|SplineComponent|IsClosedLoop (Variables|Default|GetFenceSpline))
    (LocalVariables|SetLastIndex (- _returnvalue 1))
    (else
      (LocalVariables|SetLastIndex (- _returnvalue 2))))
  (for _index (range 0 (LocalVariables|GetLastIndex))
    (bind _returnvalue_2 (AddComponent|AddSplineMeshComponent true))
    (Components|StaticMesh|SetStaticMesh _returnvalue_2 "/Game/Meshes/SM_FenceSegment.SM_FenceSegment")
    (Transformation|AttachComponentToComponent _returnvalue_2 (Variables|Default|GetFenceSpline) "None" "KeepRelative" "KeepRelative" "KeepRelative" true)
    (SplineMesh|SetStartandEnd _returnvalue_2 (.Location (Spline|GetLocationandTangentatSplinePoint _fencespline _index "Local")) (.Tangent (Spline|GetLocationandTangentatSplinePoint _fencespline _index "Local")) (.Location (Spline|GetLocationandTangentatSplinePoint (Variables|Default|GetFenceSpline) (Math|Integer|%(Integer) (+ _index 1) _returnvalue) "Local")) (.Tangent (Spline|GetLocationandTangentatSplinePoint (Variables|Default|GetFenceSpline) (Math|Integer|%(Integer) (+ _index 1) _returnvalue) "Local")) true :!class /Script/Engine.SplineMeshComponent)))

(fn CreateWheat
  (bind _returnvalue (AddComponent|AddInstancedStaticMeshComponent false (Math|Transform|MakeTransform "0, 0, 0")))
  (bind _returnvalue_2 (Components|StaticMesh|SetStaticMesh _returnvalue "/Game/Meshes/Foliage/SM_WheatField.SM_WheatField"))
  (if _returnvalue_2
    (for _index (range 0 20)
      (for _index_2 (range 0 20)
        (Components|InstancedStaticMesh|AddInstance _returnvalue (Math|Transform|MakeTransform (Math|Vector|MakeVector (* (- _index_2 10) 1e+01) (* (- _index 10) 1e+01) 0.0) (Math|Rotator|MakeRotator 0.0 0.0 (Math|Random|RandomFloatinRange 0.0 3.6e+02)) (Math|Conversions|ToVector(Float) (Math|Random|RandomFloatinRange 0.8 1.0))))))))

(fn AlignPointstoGrid)