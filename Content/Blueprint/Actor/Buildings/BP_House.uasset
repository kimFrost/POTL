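; BP_House is a house building actor that holds living slots for people.
; Its construction script rebuilds the slot list before calling the parent script, randomly filling each slot with a placeholder test person or leaving it empty.
; The person data uses a struct marked as old and deprecated.
; BeginPlay only defers to the parent, and the debug drawing call is never run.
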(event EventBeginPlay
  (|CallParentFunction))

(event Collision|EventActorBeginOverlap
  (params (OtherActor :type Actor%20Object%20Reference)))

(event EventTick
  (params (DeltaSeconds :type Float%20%28single-precision%29)))

(fn ConstructionScript
  (CallFunction|CreateLivingSpaces)
  (|CallParentFunction))

(fn CreateLivingSpaces
  (bind _livingslots (Variables|Default|GetLivingSlots))
  (Utilities|Array|Clear (Variables|Default|GetLivingSlots))
  (for _index (range 0 3)
    (if (Math|Random|RandomBool)
      (Utilities|Array|Add _livingslots (Utilities|Struct|MakeST_LivingSlot (Utilities|Struct|MakeST_PersonOLD_DEPRECATED "Test" "Test" "NewEnumerator0" (Utilities|Array|MakeArray))))
      (else
        (Utilities|Array|Add _livingslots (Utilities|Struct|MakeST_LivingSlot "(Id_2_6F765C2B44A95B41522AD1A739405AB6=,Title_5_0FE1BC8443C18FD098C11B89E71896A8=,type_8_C13570004A5F89A85F273B9A3B279CAB=NewEnumerator0,Skills_14_568BE4ED4D43FB37CBB1C3AFF907CF62=)"))))))