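; Spline mesh prop actor with a helper that lays a static mesh along a spline.
; CreateSplineMeshes adds one spline mesh component per segment, attached to the spline and shaped by the local locations and tangents of both end points.
; Closed loops get an extra segment that wraps back to the first point.
; The construction script and events are empty, so nothing in this Blueprint calls the helper.
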(event EventBeginPlay)

(event Collision|EventActorBeginOverlap
  (params (OtherActor :type Actor%20Object%20Reference)))

(event EventTick
  (params (DeltaSeconds :type Float%20%28single-precision%29)))

(fn ConstructionScript)

(fn CreateSplineMeshes
  (bind _spline (Variables|Default|GetSpline))
  (bind _spline_2 (Variables|Default|GetSpline))
  (bind _spline_3 (Variables|Default|GetSpline))
  (bind _returnvalue (Spline|GetNumberOfSplinePoints _spline_2))
  (Utilities|IsValid _spline
    (:Is%20Valid
      (if (Class|SplineComponent|IsClosedLoop _spline)
        (Variables|Default|SetLastIndex (- _returnvalue 1))
        (else
          (Variables|Default|SetLastIndex (- _returnvalue 2))))
      (for _index (range 0 (Variables|Default|GetLastIndex))
        (bind _returnvalue_2 (AddComponent|AddSplineMeshComponent (Components|GetOwner (Variables|Default|GetSpline)) true))
        (Components|StaticMesh|SetStaticMesh _returnvalue_2 (Variables|Default|GetMesh))
        (Transformation|AttachComponentToComponent _returnvalue_2 (Variables|Default|GetSpline) "None" "KeepRelative" "KeepRelative" "KeepRelative" true)
        (SplineMesh|SetStartandEnd _returnvalue_2 (.Location (Spline|GetLocationandTangentatSplinePoint _spline_3 _index "Local")) (.Tangent (Spline|GetLocationandTangentatSplinePoint _spline_3 _index "Local")) (.Location (Spline|GetLocationandTangentatSplinePoint _spline_3 (Math|Integer|%(Integer) (+ _index 1) _returnvalue) "Local")) (.Tangent (Spline|GetLocationandTangentatSplinePoint _spline_3 (Math|Integer|%(Integer) (+ _index 1) _returnvalue) "Local")) true :!class /Script/Engine.SplineMeshComponent)))))