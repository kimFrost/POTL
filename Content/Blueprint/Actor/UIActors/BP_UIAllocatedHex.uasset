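; BP_UIAllocatedHex is a UI actor that displays a Widget_HexAllocation for a hex and its owning structure.
; On BeginPlay it adds a widget component, creates the widget with the Hex and OwningStructure references, then assigns it to the component.
; Its Update function checks that the component is valid and forwards the call to the widget's own Update.
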(event EventBeginPlay
  (bind _returnvalue (AddComponent|AddWidgetComponent false))
  (bind _output_get (Variables|Default|SetWidgetComponent _returnvalue))
  (bind _returnvalue_2 (UserInterface|CreateWidget "/Game/Blueprint/UI/Widgets/Widget_HexAllocation.Widget_HexAllocation_C" 0 (Variables|Default|GetHex) (Variables|Default|GetOwningStructure)))
  (UserInterface|SetWidget _output_get _returnvalue_2))

(event Collision|EventActorBeginOverlap
  (params (OtherActor :type Actor%20Object%20Reference)))

(event EventTick
  (params (DeltaSeconds :type Float%20%28single-precision%29)))

(fn ConstructionScript)

(fn Update
  (bind _widgetcomponent (Variables|Default|GetWidgetComponent))
  (Utilities|IsValid _widgetcomponent
    (:Is%20Valid
      (bind _aswidget_hex_allocation (Utilities|Casting|CastToWidget_HexAllocation (UserInterface|GetUserWidgetObject _widgetcomponent)))
      (Default|Update _aswidget_hex_allocation))))