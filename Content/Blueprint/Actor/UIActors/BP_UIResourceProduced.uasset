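; BP_UIResourceProduced is a short-lived actor that displays a produced resource in the world through a widget component.
; On BeginPlay, if Resource is valid, it adds the component and passes Resource to Widget_ProducedResources as a single-entry queue.
; It binds to the widget's OnRemoved event and destroys itself when that fires.
; An unconnected branch using the singular Widget_ProducedResource never runs.
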(event Custom|CustomEvent_0
  (Actor|DestroyActor))

(event EventBeginPlay
  (Utilities|IsValid (Variables|Default|GetResource)
    (:Is%20Valid
      (bind _returnvalue (AddComponent|AddWidgetComponent false))
      (bind _aswidget_produced_resources (Utilities|Casting|CastToWidget_ProducedResources (UserInterface|GetUserWidgetObject _returnvalue)))
      (Variables|/Game/Blueprint/UI/Widgets/Widget_ProducedResources.Widget_ProducedResources_C|SetResourceQue _aswidget_produced_resources (Utilities|Array|MakeArray (Variables|Default|GetResource)))
      (EventDispatchers|BindEventtoOnRemoved _aswidget_produced_resources (delegate Custom|CustomEvent_0)))))

(fn ConstructionScript)