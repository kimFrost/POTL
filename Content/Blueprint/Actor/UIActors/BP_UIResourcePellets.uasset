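; BP_UIResourcePellets is an actor that displays a hex's resource pellets through a widget component.
; On BeginPlay, if its Hex reference is valid, it adds the component, passes the hex's resource info to the Widget_Pellets instance and calls Update on it.
; Disconnected leftover nodes target Widget_ProducedResource, including a removal binding to a self-destroy event, so nothing in this graph triggers that destruction.
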(event Custom|CustomEvent_0
  (Actor|DestroyActor))

(event EventBeginPlay
  (Utilities|IsValid (Variables|Default|GetHex)
    (:Is%20Valid
      (bind _returnvalue (AddComponent|AddWidgetComponent false))
      (bind _aswidget_pellets (Utilities|Casting|CastToWidget_Pellets (UserInterface|GetUserWidgetObject _returnvalue)))
      (Variables|/Game/Blueprint/UI/Widgets/Pellet/Widget_Pellets.Widget_Pellets_C|SetResourceInfo _aswidget_pellets (Variables|/Script/POTL.HexTile|GetHexResourceInfo (Variables|Default|GetHex)))
      (Default|Update _aswidget_pellets))))

(fn ConstructionScript)