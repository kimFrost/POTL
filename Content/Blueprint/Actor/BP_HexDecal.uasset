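; BP_HexDecal is a decal actor whose color can be switched by type, presumably to mark hexes.
; The construction script creates a dynamic material instance from the decal and sets its ParamColor vector parameter to an initial purple.
; ChangeType maps the given Type to a preset color on that same parameter, with a near-white fallback for unmatched types.
; It has no active BeginPlay or Tick logic.
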(event EventBeginPlay)

(event EventTick
  (params (DeltaSeconds :type Float%20%28single-precision%29)))

(fn ConstructionScript
  (bind _returnvalue (Rendering|Material|CreateDynamicMaterialInstance (Variables|Decal|GetDecal) :!class /Script/Engine.DecalComponent))
  (bind _output_get (Variables|Default|SetMaterialInstance _returnvalue))
  (Rendering|Material|SetVectorParameterValue _output_get "ParamColor" "(R=0.620317,G=0.000000,B=1.000000,A=1.000000)" :!class /Script/Engine.MaterialInstanceDynamic))

(fn ChangeType
  (params (Type :type Name))
  (bind _materialinstance (Variables|Default|GetMaterialInstance))
  (switch name Type
    (:Default
      (Rendering|Material|SetVectorParameterValue _materialinstance "ParamColor" "(R=0.876307,G=1.000000,B=0.971064,A=1.000000)" :!class /Script/Engine.MaterialInstanceDynamic))
    (:Blue
      (Rendering|Material|SetVectorParameterValue _materialinstance "ParamColor" "(R=0.000000,G=0.483937,B=1.000000,A=1.000000)" :!class /Script/Engine.MaterialInstanceDynamic))
    (:Red
      (Rendering|Material|SetVectorParameterValue _materialinstance "ParamColor" "(R=1.000000,G=0.000000,B=0.059605,A=1.000000)" :!class /Script/Engine.MaterialInstanceDynamic))
    (:Green
      (Rendering|Material|SetVectorParameterValue _materialinstance "ParamColor" "(R=0.000000,G=1.000000,B=0.153125,A=1.000000)" :!class /Script/Engine.MaterialInstanceDynamic))
    (:Pink
      (Rendering|Material|SetVectorParameterValue _materialinstance "ParamColor" "(R=1.000000,G=0.244156,B=0.570265,A=1.000000)" :!class /Script/Engine.MaterialInstanceDynamic))))