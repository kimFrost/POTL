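; Map actor that draws an arched resource-flow link between StartPoint and EndPoint and shows its Resources on hover.
; The construction script builds Out and In splines as three-point arcs, offset to either side with a raised midpoint.
; Only the Out side gets its two spline meshes and end mesh fitted; the In mesh setup is disconnected.
; Cursor-over asks HUD_Map to show the resource overlay at the arc's raised midpoint.
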(event OnBeginCursorOver(In_SplineMeshUp)
  (params (TouchedComponent :type Primitive%20Component%20Object%20Reference)))

(event OnBeginCursorOver(In_SplineMeshDown)
  (params (TouchedComponent :type Primitive%20Component%20Object%20Reference)))

(event MouseInput|EventActorBeginCursorOver
  (bind _ashud_map (Utilities|Casting|CastToHUD_Map (HUD|GetHUD (Game|GetPlayerController 0))))
  (Default|ShowResourceOverlay _ashud_map (+ (+ (/ (+ (Variables|Default|GetStartPoint) (Variables|Default|GetEndPoint)) 2.0) "0, 0,400.000000") (Transformation|GetActorLocation)) (Variables|Default|GetResources)))

(event EventBeginPlay)

(event EventActorBeginOverlap
  (params (OtherActor :type Actor%20Object%20Reference)))

(event EventTick
  (params (DeltaSeconds :type Float%20%28single-precision%29)))

(fn ConstructionScript
  (bind _startpoint (Variables|Default|GetStartPoint))
  (bind _endpoint (Variables|Default|GetEndPoint))
  (bind _out_spline (Variables|Default|GetOut_Spline))
  (bind _startpoint_2 (Variables|Default|GetStartPoint))
  (bind _endpoint_2 (Variables|Default|GetEndPoint))
  (bind _startpoint_3 (Variables|Default|GetStartPoint))
  (bind _endpoint_3 (Variables|Default|GetEndPoint))
  (bind (_location _tangent) (Spline|GetLocationandTangentatSplinePoint _out_spline 0 "Local"))
  (bind (_location_2 _tangent_2) (Spline|GetLocationandTangentatSplinePoint _out_spline 1 "Local"))
  (bind (_location_3 _tangent_3) (Spline|GetLocationandTangentatSplinePoint _out_spline 2 "Local"))
  (bind _returnvalue (Class|KismetMathLibrary|GetDirectionVector _startpoint_2 _endpoint_2))
  (bind _returnvalue_2 (+ _startpoint _endpoint))
  (bind _returnvalue_3 (/ _returnvalue_2 2.0))
  (bind _returnvalue_4 (Math|Vector|RotateVectorAroundAxis _returnvalue 9e+01 "0.000000,0.000000,1.000000"))
  (bind _returnvalue_5 (* _returnvalue_4 60))
  (bind _returnvalue_6 (+ _returnvalue_3 "0, 0,400.000000"))
  (bind _returnvalue_7 (- _returnvalue_6 _returnvalue_5))
  (Spline|ClearSplinePoints (Variables|Default|GetOut_Spline))
  (Spline|ClearSplinePoints (Variables|Default|GetIn_Spline))
  (Spline|AddSplinePoint (Variables|Default|GetOut_Spline) (- _startpoint_3 _returnvalue_5) "Local")
  (Spline|AddSplinePoint (Variables|Default|GetIn_Spline) (+ _startpoint_3 _returnvalue_5) "Local")
  (Transformation|SetRelativeLocation (Variables|Default|GetOut_MeshCatch) _returnvalue_7 false false)
  (Spline|AddSplinePoint (Variables|Default|GetOut_Spline) _returnvalue_7 "Local")
  (Spline|AddSplinePoint (Variables|Default|GetIn_Spline) (+ _returnvalue_6 _returnvalue_5) "Local")
  (Spline|AddSplinePoint (Variables|Default|GetOut_Spline) (- _endpoint_3 _returnvalue_5) "Local")
  (Spline|AddSplinePoint (Variables|Default|GetIn_Spline) (+ _endpoint_3 _returnvalue_5) "Local")
  (Utilities|FlowControl|Sequence
    (:then_0
      (SplineMesh|SetStartandEnd (Variables|Default|GetOut_SplineMeshUp) _location _tangent _location_2 _tangent_2 :!class /Script/Engine.SplineMeshComponent)
      (SplineMesh|SetStartandEnd (Variables|Default|GetOut_SplineMeshDown) _location_2 _tangent_2 _location_3 _tangent_3 :!class /Script/Engine.SplineMeshComponent)
      (Transformation|SetRelativeLocationAndRotation (Variables|Default|GetOut_EndMesh) _location_3 (Spline|GetRotationatSplinePoint _out_spline 2 "Local") false false))
    (:then_1)
    (:then_2)))