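; Island actor that hosts the map's grid plane and its resource and hex-range overlays.
; Construction applies a dynamic grid material to the plane, which BeginPlay passes to a spawned BP_OverlayDrawer before registering both with OverlayManager.
; DrawResources gathers ProviderComponents from all structures, filters them by the resource list and sends them to the drawer, clearing it when the list is empty.
; OnSpawnHexRange spawns and returns a BP_RangeDecal for given hexes.
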(event OnMapReady(TileManager))

(event Custom|CustomEvent_0
  (params (On :type Boolean))
  (bind _plane (Variables|Default|GetPlane))
  ;[1 1 1] Dev test
  (if On
    (Rendering|Material|SetMaterial _plane 0 "/Engine/EngineMaterials/WorldGridMaterial.WorldGridMaterial")
    (else
      (Rendering|Material|SetMaterial _plane 0 (Variables|Default|GetWorldDynamicMaterilInst)))))

(event EventBeginPlay
  (bind _overlaymanager (Variables|Default|GetOverlayManager))
  (Utilities|FlowControl|Sequence
    (:then_0
      (bind _returnvalue (Game|SpawnActorfromClass "/Game/Blueprint/Actor/BP_OverlayDrawer.BP_OverlayDrawer_C" (Math|Conversions|ToTransform(Vector) (Transformation|GetActorLocation)) "AlwaysSpawn" self (Variables|Default|GetWorldDynamicMaterilInst) 0))
      (Variables|Default|SetOverlayDrawer _returnvalue)
      ;[1 1 1] Setup overlay drawer blueprint ref in c++
      (Utilities|IsValid _overlaymanager
        (:Is%20Valid
          (Class|OverlayManager|Setup _overlaymanager self (Variables|Default|GetOverlayDrawer)))))))

(fn ConstructionScript
  (bind _returnvalue (Rendering|Material|CreateDynamicMaterialInstance "/Game/POTL/Stuff/M_WorldGridTest.M_WorldGridTest" :!class /Script/Engine.KismetMaterialLibrary))
  (Rendering|Material|SetMaterial (Variables|Default|GetPlane) 0 _returnvalue)
  (Variables|Default|SetWorldDynamicMaterilInst _returnvalue))

(fn GetOverlayDrawer
  (return (Variables|Default|GetOverlayDrawer)))

(fn DrawResources
  (params (ResourceList :type Map%20of%20Strings%20to%20Integers))
  (Utilities|IsValid (Variables|Default|GetTileManager)
    (:Is%20Valid
      (Utilities|IsValid (Variables|Default|GetOverlayManager)
        (:Is%20Valid
          (if (> (Utilities|Map|Length ResourceList) 0)
            (Utilities|Map|Keys ResourceList)
            (bind _outactors (Actor|GetAllActorsOfClass "/Game/Blueprint/Actor/BP_Structure.BP_Structure_C"))
            (for _array_element _outactors
              (Utilities|IsValid _array_element
                (:Is%20Valid
                  (for _array_element_2 (Actor|GetComponentsByClass _array_element "/Script/POTL.ProviderComponent")
                    (Utilities|IsValid _array_element_2
                      (:Is%20Valid
                        (Utilities|Array|Add (LocalVariables|Get_Providers) _array_element_2)))))))
            (Default|DrawProviders (Variables|Default|GetOverlayDrawer) (Class|POTLUtilFunctionLibrary|FilterProvidersbyResourceList (LocalVariables|Get_Providers) (CallFunction|ConvertResourceList ResourceList)))
            (else
              (Default|Clear (Variables|Default|GetOverlayDrawer)))))))))

(fn OnSpawnHexRange
  (params (Location :type Vector) (Hexes :type Array%20of%20Hex%20Tile%20Object%20References))
  (bind _returnvalue (Game|SpawnActorfromClass "/Game/Blueprint/Actor/BP_RangeDecal.BP_RangeDecal_C" (Math|Conversions|ToTransform(Vector) Location) "AlwaysSpawn" self Hexes 0))
  (return _returnvalue))