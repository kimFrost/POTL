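; Game instance that holds the hex map and resource state, with mouse-to-hex lookup.
; InitializeMap traces the landscape into grid points, then creates, cleans and computes rotations for the hexes.
; Mouse picking line-traces under the cursor, converts the landscape-relative hit to cube coordinates, then resolves the hex.
; ResetResources reloads from a data table and SwitchTurn forwards a turn event, while save, load and intake updates are unimplemented.
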(fn InitializeMap
  (params (Landscape :type Landscape%20Object%20Reference))
  (bind _hexwidth (Variables|Map|GetHexWidth))
  (Variables|Default|SetLandscape Landscape)
  (Variables|Calculated|SetHexHeight (* (/ (Variables|Map|GetHexWidth) (Math|Float|Sqrt 3.0)) 2.0))
  (Utilities|FlowControl|Sequence
    (:then_0
      (bind _returnvalue (Class|POTLUtilFunctionLibrary|TraceLandscape (Variables|Default|GetLandscape) (Variables|Map|GetTotalPointsX) (Variables|Map|GetTotalPointsY) (Variables|Map|GetHexWidth) "ECC_GameTraceChannel1"))
      (Variables|Map|SetPoints _returnvalue))
    (:then_1
      (bind _returnvalue_2 (Class|POTLUtilFunctionLibrary|CreateHexes (Variables|Default|GetLandscape) (Variables|Map|GetPoints) (Variables|Map|GetTotalPointsX) _hexwidth "ECC_GameTraceChannel1"))
      (bind _returnvalue_3 (Class|POTLUtilFunctionLibrary|CleanHexes _returnvalue_2))
      (bind _returnvalue_4 (Class|POTLUtilFunctionLibrary|CalcHexesRot _returnvalue_3 _hexwidth))
      (Variables|Map|SetHexes _returnvalue_4)
      (bind _output_get (LocalVariables|Set_MapInitialized true))
      (return _output_get))))

(fn ResetResources
  (bind _outrownames (DataTable|GetDataTableRowNames "/Game/Resources/Data_Resources.Data_Resources"))
  (Utilities|Array|Clear (Variables|Resources|GetResources))
  (for _array_element _outrownames
    (bind _returnvalue (Utilities|GetDataTableRow "/Game/Resources/Data_Resources.Data_Resources" _array_element)
      (:then
        (Utilities|Array|Add (Variables|Resources|GetResources) _returnvalue)))))

(fn SaveGame)

(fn LoadGame)

(fn SwitchTurn
  (params (direction :type Integer :default 0))
  (Default|CallTurnSwitched direction))

(fn UpdateResourceIntakes)

(fn LoadMap)

(fn MousePostoCube
  (bind _returnvalue (Game|GetPlayerController 0))
  (bind (_worldlocation _worlddirection) (Game|Player|ConvertMouseLocationToWorldSpace _returnvalue))
  (bind (_outhit _returnvalue_2) (Collision|LineTraceForObjects _worldlocation (+ _worldlocation (* _worlddirection 5e+04)) (Utilities|Array|MakeArray "ObjectTypeQuery7") false 0 "None"))
  (if _returnvalue_2
    (bind _returnvalue_3 (Class|POTLUtilFunctionLibrary|LocationtoCube (Variables|Map|GetTotalPointsX) (Variables|Map|GetHexWidth) (Variables|Calculated|GetHexHeight) (- (.Location (Collision|BreakHitResult _outhit)) (Transformation|GetActorLocation (Variables|Default|GetLandscape))))))
  (return _returnvalue_2 _returnvalue_3))

(fn MousePostoHex
  (bind (_found _cube) (CallFunction|MousePostoCube))
  (if _found
    (bind _returnvalue (Class|POTLUtilFunctionLibrary|CubetoHex _cube (Variables|Map|GetHexes) (Variables|Map|GetTotalPointsX)))
    (return _found _returnvalue)))