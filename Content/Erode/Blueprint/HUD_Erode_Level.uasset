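; Prototype HUD for the Erode level that places a hex tile where the player clicks.
; BeginPlay enables input and spawns one BP_Hextile, which each left click moves to the hit of a deprojected mouse trace, with scale and an impact-point-derived roll.
; DrawHUD caches screen size and draws placeholder text.
; Debug traces and prints remain, alongside disconnected screen-offset experiments and a stray construction-script trace.
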(event EventDrawHUD
  (params (SizeX :type Integer) (SizeY :type Integer))
  (Variables|Default|SetScreenDimensions (Math|Vector2D|MakeVector2D (Math|Conversions|ToFloat(Integer) SizeX) (Math|Conversions|ToFloat(Integer) SizeY)))
  (HUD|DrawText "TESTING" "(R=0.111375,G=0.111658,B=0.165000,A=1.000000)" 0.0 0.0 0 1.0 false))

(event EventBeginPlay
  (Input|EnableInput (Game|GetPlayerController 0))
  (bind _returnvalue (Game|SpawnActorfromClass "/Game/Erode/Blueprint/Actors/BP_Hextile.BP_Hextile_C" (Math|Transform|MakeTransform "0, 0, 0") false 0))
  (Variables|Default|SetSelectedTile _returnvalue))

(event Input|MouseEvents|LeftMouseButton
  (bind _returnvalue (Game|GetPlayerController 0))
  (bind (_worldlocation _worlddirection) (Game|Player|ConvertMouseLocationToWorldSpace _returnvalue))
  (:Pressed
    (bind (_outhit _returnvalue_2) (Collision|LineTraceByChannel _worldlocation (+ _worldlocation (* _worlddirection 1e+04)) "TraceTypeQuery1" true 0 "Persistent"))
    (if _returnvalue_2
      (Development|PrintString (Utilities|String|ToString(Vector) (.Location (Collision|BreakHitResult _outhit))))
      (Transformation|SetActorTransform (Variables|Default|GetSelectedTile) (Math|Transform|MakeTransform (.Location (Collision|BreakHitResult _outhit)) (Class|KismetMathLibrary|MakeRot 0.0 0.0 (+ (.Roll (Class|KismetMathLibrary|BreakRot (Math|Conversions|RotationFromXVector (.ImpactPoint (Collision|BreakHitResult _outhit))))) 0.0)) "1.400000,1.400000,1.400000"))
      (Development|PrintString (Utilities|String|ToString(Vector) (.ImpactPoint (Collision|BreakHitResult _outhit)))))))

(fn ConstructionScript
  (Collision|LineTraceByChannel "0, 0, 0" "0, 0, 0" "TraceTypeQuery1" false 0 "None"))