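; Visualizer actor that draws an arched link between a FromStructure and a ToStructure, presumably to show allocated resources.
; On construction it clears its spline and, if both structures are valid, moves to the source and adds points at the start, a raised midpoint and the target.
; Two spline meshes, SplineMeshUp and SplineMeshDown, are stretched along the rising and falling halves using the spline's tangents.
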(event EventBeginPlay)

(event Collision|EventActorBeginOverlap
  (params (OtherActor :type Actor%20Object%20Reference)))

(event EventTick
  (params (DeltaSeconds :type Float%20%28single-precision%29)))

(fn ConstructionScript
  (bind _fromstructure (Variables|Default|GetFromStructure))
  (bind _spline (Variables|Default|GetSpline))
  (bind _tostructure (Variables|Default|GetToStructure))
  (bind (_location _tangent) (Spline|GetLocationandTangentatSplinePoint _spline 0 "Local"))
  (bind (_location_2 _tangent_2) (Spline|GetLocationandTangentatSplinePoint _spline 1 "Local"))
  (bind (_location_3 _tangent_3) (Spline|GetLocationandTangentatSplinePoint _spline 2 "Local"))
  (Spline|ClearSplinePoints (Variables|Default|GetSpline) true)
  (Utilities|IsValid _fromstructure
    (:Is%20Valid
      (Utilities|IsValid _tostructure
        (:Is%20Valid
          (bind _output_get (Variables|Default|SetStartPos (Transformation|GetActorLocation _fromstructure)))
          (Variables|Default|SetEndPos (Transformation|GetActorLocation _tostructure))
          (Transformation|SetActorLocation _output_get false true)
          (Spline|AddSplinePoint (Variables|Default|GetSpline) (Math|Vector|MakeVector 0.0 0.0 0.0) "Local" true)
          (Spline|AddSplinePoint (Variables|Default|GetSpline) (+ (/ (- (Variables|Default|GetEndPos) (Variables|Default|GetStartPos)) 2.0) "0, 0,250.000000") "Local" true)
          (Spline|AddSplinePoint (Variables|Default|GetSpline) (Transformation|GetActorLocation (Variables|Default|GetToStructure)) "World" true)
          (SplineMesh|SetStartandEnd (Variables|Default|GetSplineMeshUp) _location _tangent _location_2 _tangent_2 true :!class /Script/Engine.SplineMeshComponent)
          (SplineMesh|SetStartandEnd (Variables|Default|GetSplineMeshDown) _location_2 _tangent_2 _location_3 _tangent_3 true :!class /Script/Engine.SplineMeshComponent))))))