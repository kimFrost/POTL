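; CRT_WorldGrid is a canvas render target that draws a hex texture, apparently as groundwork for a world grid map.
; On update it draws a single Hex texture at the canvas midpoint, sized by dividing the canvas dimensions by fixed divisors.
; A loop over valid Hexes and the math to map their locations relative to the canvas are present but unconnected, so no grid is drawn.
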(event EventUpdate
  (params (Canvas :type Canvas%20Object%20Reference) (Width :type Integer) (Height :type Integer))
  (bind _returnvalue (Math|Conversions|ToFloat(Integer) Height))
  (bind _returnvalue_2 (Math|Conversions|ToFloat(Integer) Width))
  (Canvas|DrawTexture Canvas "/Game/Textures/Hex/hex.hex" (Math|Vector2D|MakeVector2D (/ _returnvalue_2 2.0) (/ _returnvalue 2.0)) (Math|Vector2D|MakeVector2D (/ _returnvalue_2 (Math|Float|MakeLiteralFloat 255.0)) (/ _returnvalue (Math|Float|MakeLiteralFloat 294.0))) "(X=0.000000,Y=0.000000)" "(X=1.000000,Y=1.000000)" "(R=1.000000,G=1.000000,B=1.000000,A=1.000000)" "BLEND_Translucent" 0.0 "(X=0.500000,Y=0.500000)"))