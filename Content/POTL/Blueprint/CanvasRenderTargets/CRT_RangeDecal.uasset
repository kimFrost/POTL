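; Canvas render target, apparently for a hex range decal, that paints a hex texture onto its canvas.
; DrawHexes stores a hex color list and calls UpdateResource to trigger a redraw.
; The Update event prints a debug message and stretches a single Hex texture over the whole target, ignoring the stored list.
; The per-hex loop, material draw and test line are disconnected, so the asset looks unfinished.
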(event EventUpdate
  (params (Canvas :type Canvas%20Object%20Reference) (Width :type Integer) (Height :type Integer))
  (Development|PrintString "DRAW!!!")
  (Canvas|DrawTexture :self Canvas :RenderTexture "/Game/Textures/Hex/hex.hex" :ScreenSize (Math|Vector2D|MakeVector2D (Math|Conversions|ToFloat(Integer) Width) (Math|Conversions|ToFloat(Integer) Height)) :CoordinateSize "(X=1.000000,Y=1.000000)"))

(fn DrawHexes
  (params (HexColorList :type Array%20of%20Hex%20Linear%20Color%20Structures))
  (Variables|Default|SetHexColorList HexColorList)
  (Class|CanvasRenderTarget2D|UpdateResource))