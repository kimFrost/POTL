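; BP_TestWorldGrid is a test actor that feeds hex tile data to a world grid material through a texture.
; Its construction script applies a dynamic M_WorldGridTest material to the static mesh and binds a one-pixel-high RT_WorldGrid canvas render target as TileStates.
; It fills an array with new HexTile objects, hands it to the render target and triggers a redraw.
; The event graph holds no active logic.
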(event EventBeginPlay)

(event Collision|EventActorBeginOverlap
  (params (OtherActor :type Actor%20Object%20Reference)))

(event EventTick
  (params (DeltaSeconds :type Float%20%28single-precision%29)))

(fn ConstructionScript
  (bind _returnvalue (Rendering|Material|CreateDynamicMaterialInstance "/Game/POTL/Stuff/M_WorldGridTest.M_WorldGridTest" :!class /Script/Engine.KismetMaterialLibrary))
  (Rendering|Material|SetMaterial (Variables|Default|GetStaticMesh) 0 _returnvalue)
  (bind _returnvalue_2 (CanvasRenderTarget2D|CreateCanvasRenderTarget2D "/Game/POTL/Stuff/RT_WorldGrid.RT_WorldGrid_C" 100 1))
  (Variables|Default|SetRTWorldGrid _returnvalue_2)
  (Rendering|Material|SetTextureParameterValue _returnvalue "TileStates" _returnvalue_2)
  (bind _asrt_world_grid (Utilities|Casting|CastToRT_WorldGrid _returnvalue_2))
  (for _index (range 0 100)
    (bind _returnvalue_3 (Game|ConstructObjectfromClass "/Script/POTL.HexTile" self))
    (Utilities|Array|Add (LocalVariables|Get_Tiles) _returnvalue_3))
  (Variables|/Game/POTL/Stuff/RT_WorldGrid.RT_WorldGrid_C|SetTiles _asrt_world_grid (LocalVariables|Get_Tiles))
  (Class|CanvasRenderTarget2D|UpdateResource _returnvalue_2))